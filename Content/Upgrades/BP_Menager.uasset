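; Game manager Blueprint that holds Score and Health and handles building purchases and a shield upgrade.
; On BeginPlay it creates the upgrades widget and enables mouse input for game and UI.
; Buying a building looks up its cost by enum name in a data table and only deducts affordable Score.
; The shield takes its duration from the "Freze" upgrade row, using a Timeline as a timer during which RemoveHealth is blocked.
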(event Custom|Buy%20building
  (params (Building%20type :type Building_Types%20Enum :default "NewEnumerator0"))
  (bind _returnvalue (Utilities|GetDataTableRow "/Game/Upgrades/Data/Buildings.Buildings" (Utilities|String|StringToName (Utilities|String|EnumtoString Building%20type)))
    (:then
      (if (>= (Variables|Default|GetScore) (.Cost (Utilities|Struct|BreakS_Building _returnvalue)))
        (Variables|Default|SetScore (- (Variables|Default|GetScore) (.Cost (Utilities|Struct|BreakS_Building _returnvalue))))))))

(event Custom|Activate%20shield
  (bind _returnvalue (Utilities|GetDataTableRow "/Game/Upgrades/Data/Upgrades.Upgrades" "Freze")
    (:then
      (Components|Timeline|SetTimelineLength (Variables|Default|GetTimeline) (Math|Conversions|ToFloat(Integer) (.Lenght (Utilities|Struct|BreakS_Upgrades _returnvalue))))
      (Variables|Default|SetShield%20Active%20? true)
      (Timeline|Timeline PlayFromStart
        (:Finished
          (Variables|Default|SetShield%20Active%20? false))))))

(event EventBeginPlay
  (bind _returnvalue (Game|GetPlayerController 0))
  (bind _returnvalue_2 (UserInterface|CreateWidget "/Game/Upgrades/W_UpgradesUI.W_UpgradesUI_C"))
  (UserInterface|Viewport|AddtoViewport _returnvalue_2 0)
  (Variables|/Script/Engine.PlayerController|SetbShowMouseCursor _returnvalue true)
  (Input|SetInputModeGameandUI _returnvalue 0 "DoNotLock" true false))

(fn ConstructionScript)

(fn AddScore
  (params (INT :type Integer))
  (Variables|Default|SetScore (+ INT (Variables|Default|GetScore))))

(fn RemoveHealth
  (params (INT :type Integer))
  (if (not (Variables|Default|GetShield%20Active%20?))
    (Variables|Default|SetHealth (- (Variables|Default|GetHealth) INT))))