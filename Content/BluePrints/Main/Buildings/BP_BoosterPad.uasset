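; BP_BoosterPad is a booster pad that pushes the main ball and enemies along its right vector.
; Box overlap events maintain a list of actors on the pad, which Tick loops over to apply continuous force.
; The main ball gets a much stronger push and replays a 2D booster sound every tick.
; Enemies get a weaker push, except one enemy type, which is left unaffected.
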(event OnComponentBeginOverlap(Box)
  (params (OverlappedComponent :type Primitive%20Component%20Object%20Reference) (OtherActor :type Actor%20Object%20Reference) (OtherComp :type Primitive%20Component%20Object%20Reference) (OtherBodyIndex :type Integer) (bFromSweep :type Boolean) (SweepResult :type Hit%20Result%20Structure%20%28by%20ref%29))
  (Utilities|Array|Add (Variables|Default|GetObjectList) OtherActor))

(event OnComponentEndOverlap(Box)
  (params (OverlappedComponent :type Primitive%20Component%20Object%20Reference) (OtherActor :type Actor%20Object%20Reference) (OtherComp :type Primitive%20Component%20Object%20Reference) (OtherBodyIndex :type Integer))
  (Utilities|Array|RemoveItem (Variables|Default|GetObjectList) OtherActor))

(event EventBeginPlay)

(event Collision|EventActorBeginOverlap
  (params (OtherActor :type Actor%20Object%20Reference)))

(event EventTick
  (params (DeltaSeconds :type Float%20%28single-precision%29))
  (for _array_element (Variables|Default|GetObjectList)
    (bind _asbp_main_ball (Utilities|Casting|CastToBP_MainBall _array_element)
      (:then
        (Physics|AddForce (Variables|/Game/BluePrints/Main/BP_MainBall.BP_MainBall_C|GetSphere _asbp_main_ball) (* (Transformation|GetActorRightVector self) 400000) "None" false)
        (Audio|PlaySound2D "/Game/BluePrints/Main/Sounds/SC_Booster.SC_Booster" 1.0 1.0 0.0 0 0))
      (:CastFailed
        (bind _asbp_enemy (Utilities|Casting|CastToBP_Enemy _array_element))
        (if (Utilities|Enum|NotEqual(Enum) (Variables|/Game/BluePrints/Main/Enemy/BP_Enemy.BP_Enemy_C|GetType _asbp_enemy) "NewEnumerator1")
          (Physics|AddForce (Variables|/Game/BluePrints/Main/Enemy/BP_Enemy.BP_Enemy_C|GetSphere _asbp_enemy) (* (Transformation|GetActorRightVector self) 70000) "None" false))))))

(fn ConstructionScript)