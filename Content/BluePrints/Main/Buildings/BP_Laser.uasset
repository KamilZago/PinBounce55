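; BP_Laser is a laser building that damages enemies crossing its beam and wears out with use.
; It reads its starting Durability from the Laser row of the Buildings data table on BeginPlay.
; While Active, each enemy beam overlap calls Dmg on the BP_Enemy and costs one Durability.
; UpdateLaser matches beam visibility to Active and destroys the actor when Durability reaches zero.
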(event OnComponentBeginOverlap(Laser_beam)
  (params (OverlappedComponent :type Primitive%20Component%20Object%20Reference) (OtherActor :type Actor%20Object%20Reference) (OtherComp :type Primitive%20Component%20Object%20Reference) (OtherBodyIndex :type Integer) (bFromSweep :type Boolean) (SweepResult :type Hit%20Result%20Structure%20%28by%20ref%29))
  (bind _asbp_enemy (Utilities|Casting|CastToBP_Enemy OtherActor))
  (if (Variables|Default|GetActive%20?)
    (Default|Dmg _asbp_enemy)
    (Math|Integer|DecrementInt (Variables|Default|GetDurability)
      (:%20%20
        (CallFunction|UpdateLaser)))))

(event Custom|Update%20laser
  (Rendering|SetVisibility (Variables|Default|GetLaser_beam) (Variables|Default|GetActive%20?) false)
  (if (== (Variables|Default|GetDurability) 0)
    (Actor|DestroyActor)))

(event EventBeginPlay
  (bind _returnvalue (Utilities|GetDataTableRow "/Game/Upgrades/Data/Buildings.Buildings" "Laser")
    (:then
      (Variables|Default|SetDurability (.Durability (Utilities|Struct|BreakS_Building _returnvalue)))
      (CallFunction|UpdateLaser))))

(fn ConstructionScript)