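; BP_Wall is a destructible wall building that loses durability when hit.
; On BeginPlay it reads current and maximum durability from the "Wall" row of the Buildings data table.
; Each component hit on its static mesh prints a debug string, subtracts one durability and spawns a high, medium or low HP effect at the mesh based on the remaining fraction.
; The actor destroys itself when durability runs out.
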(event OnComponentHit(StaticMesh)
  (params (HitComponent :type Primitive%20Component%20Object%20Reference) (OtherActor :type Actor%20Object%20Reference) (OtherComp :type Primitive%20Component%20Object%20Reference) (NormalImpulse :type Vector :default "0, 0, 0") (Hit :type Hit%20Result%20Structure%20%28by%20ref%29))
  (bind _staticmesh (Variables|Default|GetStaticMesh))
  (bind _durability (Variables|Default|GetDurability))
  (bind _maxdurability (Variables|Default|Getmaxdurability))
  (bind _returnvalue (Transformation|GetWorldTransform _staticmesh))
  (bind _returnvalue_2 (/ _durability _maxdurability))
  (bind (_location _rotation) (Math|Transform|BreakTransform _returnvalue))
  (Development|PrintString "Hello")
  (Variables|Default|Setdurability (- (Variables|Default|Getdurability) 1))
  (if (<= _returnvalue_2 0.33)
    (Niagara|SpawnSystematLocation "/Game/BluePrints/Main/Particle/ES_BuildingLowHP.ES_BuildingLowHP" _location _rotation)
    (if (<= (Variables|Default|Getdurability) 0) :!label _label
      (Actor|DestroyActor))
    (elif (<= _returnvalue_2 0.66)
      (Niagara|SpawnSystematLocation "/Game/BluePrints/Main/Particle/ES_BuildingMediumHP.ES_BuildingMediumHP" _location _rotation)
      (else
        (Niagara|SpawnSystematLocation "/Game/BluePrints/Main/Particle/ES_BuildingHighHP.ES_BuildingHighHP" _location _rotation)
        (goto _label)))))

(event EventBeginPlay
  (bind _returnvalue (Utilities|GetDataTableRow "/Game/Upgrades/Data/Buildings.Buildings" "Wall")
    (:then
      (Variables|Default|SetDurability (.Durability (Utilities|Struct|BreakS_Building _returnvalue)))
      (Variables|Default|Setmaxdurability (Math|Conversions|ToFloat(Integer) (.Durability (Utilities|Struct|BreakS_Building _returnvalue)))))))

(event Collision|EventActorBeginOverlap
  (params (OtherActor :type Actor%20Object%20Reference)))

(event EventTick
  (params (DeltaSeconds :type Float%20%28single-precision%29)))

(fn ConstructionScript)