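; BP_Bouncer is a bumper that knocks the main ball and enemies away on contact.
; When its static mesh is hit, it casts the other actor to BP_MainBall or BP_Enemy and applies a force to its sphere, pointing away from the bouncer's center.
; The ball receives a much stronger push than enemies.
; Either hit restarts a timeline that animates the mesh's uniform scale as visual feedback.
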(event OnComponentHit(StaticMesh)
  (params (HitComponent :type Primitive%20Component%20Object%20Reference) (OtherActor :type Actor%20Object%20Reference) (OtherComp :type Primitive%20Component%20Object%20Reference) (NormalImpulse :type Vector :default "0, 0, 0") (Hit :type Hit%20Result%20Structure%20%28by%20ref%29))
  (bind _asbp_main_ball (Utilities|Casting|CastToBP_MainBall OtherActor)
    (:then
      (Physics|AddForce (Variables|/Game/BluePrints/Main/BP_MainBall.BP_MainBall_C|GetSphere _asbp_main_ball) (* (Math|Vector|Normalize (- (Transformation|GetWorldLocation (Variables|/Game/BluePrints/Main/BP_MainBall.BP_MainBall_C|GetSphere _asbp_main_ball)) (Transformation|GetActorLocation self)) 0.001) 40000000) "None" false)
      (bind _newtrack_0 (Timeline|Timeline PlayFromStart)
        (:Update
          (Transformation|SetRelativeScale3D (Variables|Default|GetStaticMesh) (Math|Conversions|ToVector(Float) (+ _newtrack_0 2.0))))))
    (:CastFailed
      (bind _asbp_enemy (Utilities|Casting|CastToBP_Enemy OtherActor))
      (Physics|AddForce (Variables|/Game/BluePrints/Main/Enemy/BP_Enemy.BP_Enemy_C|GetSphere _asbp_enemy) (* (Math|Vector|Normalize (- (Transformation|GetWorldLocation (Variables|/Game/BluePrints/Main/Enemy/BP_Enemy.BP_Enemy_C|GetSphere _asbp_enemy)) (Transformation|GetActorLocation self)) 0.001) 7000000) "None" false)
      (Timeline|Timeline PlayFromStart))))

(event EventBeginPlay)

(event Collision|EventActorBeginOverlap
  (params (OtherActor :type Actor%20Object%20Reference)))

(event EventTick
  (params (DeltaSeconds :type Float%20%28single-precision%29)))

(fn ConstructionScript)