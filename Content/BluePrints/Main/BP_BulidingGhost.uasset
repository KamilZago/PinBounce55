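; BP_BulidingGhost is a placement ghost that previews the selected building type, either a Bouncer or a Booster Pad.
; ChangeBulidng shows the Cone and toggles between a static mesh for the Bouncer and three cube components for the Booster Pad.
; For the Bouncer, it swaps in the Bumper mesh and overrides every material slot with the ghost material.
; It starts as a Bouncer on BeginPlay, and an Invisible event hides all its components.
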(event Custom|ChangeBulidng
  (params (BulidingType :type Building_Types%20Enum :default "NewEnumerator0"))
  (Rendering|SetVisibility (Variables|Default|GetCone) true false)
  (switch Utilities|FlowControl|Switch|SwitchonBuilding_Types BulidingType
    (:NewEnumerator0
      (Variables|Default|SetCurrentStaticMesh "/Game/Models/Bumper.Bumper")
      (CallFunction|ChangeMaterials)
      (Rendering|SetVisibility (Variables|Default|GetCube1) false false)
      (Rendering|SetVisibility (Variables|Default|GetStaticMesh) true false))
    (:NewEnumerator2
      (Rendering|SetVisibility (Variables|Default|GetCube1) true false)
      (Rendering|SetVisibility (Variables|Default|GetStaticMesh) false false))))

(event Custom|ChangeMaterials
  (bind _staticmesh (Variables|Default|GetStaticMesh))
  (Components|StaticMesh|SetStaticMesh _staticmesh (Variables|Default|GetCurrentStaticMesh))
  (for _index (range 0 (- (Utilities|Array|Length (Rendering|Material|GetMaterials _staticmesh)) 1))
    (Rendering|Material|SetMaterial _staticmesh _index "/Game/Materials/M_BulidingGhost.M_BulidingGhost")))

(event Custom|Invisible
  (Rendering|SetVisibility (Variables|Default|GetCube1) false false))

(event EventBeginPlay
  (CallFunction|ChangeBulidng "NewEnumerator0"))

(fn ConstructionScript)