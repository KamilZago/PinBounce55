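; Player controller for a paddle-based game with building placement, routing Enhanced Input to the level's BP_Paddle and a pause-menu toggle.
; BeginPlay creates the health and HUD widgets, sets input and frame-rate settings, and caches the paddle, character and building ghost.
; In building mode, a cursor trace aligns the ghost to BP_Table's surface normal.
; Left-click calls BP_Menager's purchase and placement (only Bouncer spawns) without checking building mode or purchase success.
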(event Custom|OnMouseMove
  (bind _returnvalue (Game|GetPlayerController 0))
  (bind _bp_buliding_ghost (Variables|Default|GetBP%20Buliding%20Ghost))
  (bind (_locationx _locationy) (Game|Player|GetMousePosition _returnvalue))
  (bind (_worldlocation _worlddirection) (Class|PlayerController|DeprojectScreenPositiontoWorld _returnvalue _locationx _locationy))
  (if (Variables|Default|Get?BuildingMode)
    (bind _outhit (Collision|LineTraceForObjects _worldlocation (+ _worldlocation (* _worlddirection 100000000)) (Utilities|Array|MakeArray "ObjectTypeQuery6") false 0 "None"))
    (Utilities|Casting|CastToBP_Table (.HitActor (Collision|BreakHitResult _outhit))
      (:then
        (Rendering|SetActorHiddenInGame _bp_buliding_ghost false)
        (bind _output_get (Variables|Default|SetBuildingSpawnTransform (Math|Transform|MakeTransform (.Location (Collision|BreakHitResult _outhit)) (Math|Rotator|MakeRotator (.Roll (Math|Rotator|BreakRotator (Math|Rotator|FindLookatRotation (Math|Vector|MakeVector 0.0 0.0 0.0) (.ImpactNormal (Collision|BreakHitResult _outhit))))) (+ (.Pitch (Math|Rotator|BreakRotator (Math|Rotator|FindLookatRotation (Math|Vector|MakeVector 0.0 0.0 0.0) (.ImpactNormal (Collision|BreakHitResult _outhit))))) -9e+01) (.Yaw (Math|Rotator|BreakRotator (Math|Rotator|FindLookatRotation (Math|Vector|MakeVector 0.0 0.0 0.0) (.ImpactNormal (Collision|BreakHitResult _outhit)))))))))
        (Transformation|SetActorTransform _bp_buliding_ghost _output_get))
      (:CastFailed
        (Rendering|SetActorHiddenInGame _bp_buliding_ghost true)))))

(event Custom|ChangeBulidingType
  (params (BuildingType :type Building_Types%20Enum :default "NewEnumerator0"))
  (Default|ChangeBulidng (Variables|Default|GetBP%20Buliding%20Ghost) BuildingType))

(event Custom|PlaceBuilding
  (switch Utilities|FlowControl|Switch|SwitchonBuilding_Types (Variables|Default|GetCurrentBulidingType)
    (:NewEnumerator0
      (Variables|Default|SetCurrentBuildingClass "/Game/BluePrints/Main/Buildings/BP_Bouncer.BP_Bouncer_C")
      (Game|SpawnActorfromClass (Variables|Default|GetCurrentBuildingClass) (Variables|Default|GetBuildingSpawnTransform) "Undefined" "MultiplyWithRoot" 0 0)
      (Rendering|SetActorHiddenInGame (Variables|Default|GetBP%20Buliding%20Ghost) true))))

(event Input|EnhancedActionEvents|EnhancedInputActionIA_Pause
  (params (ActionValue :type Boolean) (ElapsedSeconds :type Float%20%28double-precision%29) (TriggeredSeconds :type Float%20%28double-precision%29) (InputAction :type Input%20Action%20Object%20Reference :default "/Game/Input/IA_Pause.IA_Pause"))
  (:Started
    (if (Game|IsGamePaused)
      (Game|SetGamePaused false)
      (Widget|RemovefromParent (Variables|Default|GetWB%20Settings))
      (Variables|Default|SetWB%20Settings 0)
      (Variables|/Script/Engine.PlayerController|SetbShowMouseCursor (Game|GetPlayerController 0) false)
      (else
        (Game|SetGamePaused true)
        (bind _returnvalue (UserInterface|CreateWidget "/Game/UI/WB_Settings.WB_Settings_C"))
        (UserInterface|Viewport|AddtoViewport _returnvalue 0)
        (bind _output_get (Variables|Default|SetWB%20Settings _returnvalue))
        (Variables|/Game/UI/WB_Settings.WB_Settings_C|Set?IsPauseMenu _output_get true)
        (Variables|/Script/Engine.PlayerController|SetbShowMouseCursor (Game|GetPlayerController 0) true)))))

(event Input|EnhancedActionEvents|EnhancedInputActionIA_LeftPaddle
  (params (ActionValue :type Boolean) (ElapsedSeconds :type Float%20%28double-precision%29) (TriggeredSeconds :type Float%20%28double-precision%29) (InputAction :type Input%20Action%20Object%20Reference :default "/Game/Input/IA_LeftPaddle.IA_LeftPaddle"))
  (bind _paddle (Variables|Default|GetPaddle))
  ;[0.15 0 0 0.5] Paddles
  (:Started
    (bind _asbp_paddle (Utilities|Casting|CastToBP_Paddle _paddle))
    (Default|LeftPaddle _asbp_paddle))
  (:Completed
    (bind _asbp_paddle_2 (Utilities|Casting|CastToBP_Paddle _paddle))
    (Default|LeftPaddleReset _asbp_paddle_2)))

(event Input|EnhancedActionEvents|EnhancedInputActionIA_RightPaddle
  (params (ActionValue :type Boolean) (ElapsedSeconds :type Float%20%28double-precision%29) (TriggeredSeconds :type Float%20%28double-precision%29) (InputAction :type Input%20Action%20Object%20Reference :default "/Game/Input/IA_RightPaddle.IA_RightPaddle"))
  (bind _paddle (Variables|Default|GetPaddle))
  ;[0.15 0 0 0.5] Paddles
  (:Started
    (bind _asbp_paddle (Utilities|Casting|CastToBP_Paddle _paddle))
    (Default|RightPaddle _asbp_paddle))
  (:Completed
    (bind _asbp_paddle_2 (Utilities|Casting|CastToBP_Paddle _paddle))
    (Default|RightPaddleReset _asbp_paddle_2)))

(event EventBeginPlay
  (bind _returnvalue (UserInterface|CreateWidget "/Game/BluePrints/Main/WB_Health.WB_Health_C"))
  (UserInterface|Viewport|AddtoViewport _returnvalue 0)
  (Utilities|FlowControl|Sequence
    (:then_0
      (bind _outactors (Actor|GetAllActorsOfClass "/Game/BluePrints/Main/Paddle/BP_Paddle.BP_Paddle_C"))
      (bind _asbp_paddle (Utilities|Casting|CastToBP_Paddle (Utilities|Array|Get(acopy) _outactors)))
      (Variables|Default|SetPaddle _asbp_paddle))
    (:then_1
      (Input|SetInputModeGameandUI self 0 "DoNotLock" true false)
      (bind _returnvalue_2 (Settings|GetGameUserSettings))
      (Class|GameUserSettings|SetFrameRateLimit _returnvalue_2 0.0)
      (Class|GameUserSettings|SaveSettings _returnvalue_2)
      (Input|AddMappingContext (PlayerController|LocalPlayerSubsystems|GetEnhancedInputLocalPlayerSubsystem self) "/Game/Input/IMC_Main.IMC_Main" 0 "(bIgnoreAllPressedKeysUntilRelease=True,bForceImmediately=False,bNotifyUserSettings=False)")
      (bind _asbp_character (Utilities|Casting|CastToBP_Character (Game|Player|GetPlayerPawn 0)))
      (Variables|Default|SetBP%20Character _asbp_character)
      (bind _returnvalue_3 (UserInterface|CreateWidget "/Game/UI/WB_HUD.WB_HUD_C"))
      (UserInterface|Viewport|AddtoViewport _returnvalue_3 0))
    (:then_2
      (bind _outactors_2 (Actor|GetAllActorsOfClass "/Game/BluePrints/Main/BP_BulidingGhost.BP_BulidingGhost_C"))
      (Variables|Default|SetBP%20Buliding%20Ghost (Utilities|Array|Get(acopy) _outactors_2)))))

(event EventTick
  (params (DeltaSeconds :type Float%20%28single-precision%29)))

(event Input|MouseEvents|LeftMouseButton
  (params (Key :type Key%20Structure :default "None"))
  ;[0.15 0.15 0.15 0.5] Mouse click maniger
  (:Pressed
    (bind _returnvalue (Actor|GetActorOfClass "/Game/Upgrades/BP_Menager.BP_Menager_C"))
    (Default|BuyBuilding _returnvalue (Variables|Default|GetCurrentBulidingType))
    (CallFunction|PlaceBuilding)
    (Variables|Default|Set?BuildingMode false)))

(event Input|MouseEvents|RightMouseButton
  (params (Key :type Key%20Structure :default "None"))
  ;[0.15 0.15 0.15 0.5] Mouse click maniger
  (:Pressed
    (Variables|Default|Set?BuildingMode false)))

(event Input|MouseEvents|Mouse2D
  (params (AxisValue :type Vector :default "0, 0, 0"))
  (CallFunction|OnMouseMove))

(fn ConstructionScript)