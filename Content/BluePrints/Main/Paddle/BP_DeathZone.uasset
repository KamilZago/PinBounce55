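; Death zone trigger that destroys any main ball entering it and handles the respawn of a full-size ball.
; Cube overlap plays a death sound and destroys the ball, continuing only if its root Z scale was exactly 1.
; For such balls, a timeline feeds a countdown widget, then calls SpawnBall on the first BP_BallSpawn in the level and removes the widget.
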(event OnComponentBeginOverlap(Cube)
  (params (OverlappedComponent :type Primitive%20Component%20Object%20Reference) (OtherActor :type Actor%20Object%20Reference) (OtherComp :type Primitive%20Component%20Object%20Reference) (OtherBodyIndex :type Integer) (bFromSweep :type Boolean) (SweepResult :type Hit%20Result%20Structure%20%28by%20ref%29))
  (bind _asbp_main_ball (Utilities|Casting|CastToBP_MainBall OtherActor))
  (bind _output_get (Variables|Default|Set?IsBig (== (.Z (Math|Vector|BreakVector (Transformation|GetWorldScale (Variables|/Game/BluePrints/Main/BP_MainBall.BP_MainBall_C|GetDefaultSceneRoot _asbp_main_ball)))) 1.0)))
  (Audio|PlaySound2D "/Game/BluePrints/Main/Sounds/SC_BallDeath.SC_BallDeath" 1.0 1.0 0.0 0 0)
  ;[0.15 0 0 0.5] Zniszczenie i respawn nowej pilki i timer
  (Actor|DestroyActor _asbp_main_ball)
  (if _output_get
    (Utilities|FlowControl|Sequence
      (:then_0
        (bind _returnvalue (UserInterface|CreateWidget "/Game/BluePrints/Main/Paddle/WB_DeathTimer.WB_DeathTimer_C"))
        (bind _output_get_2 (Variables|Default|SetDeath%20Timer _returnvalue))
        (UserInterface|Viewport|AddtoViewport _returnvalue 0))
      (:then_1
        (bind _death (Timeline|DeathTimer PlayFromStart)
          (:Update
            (Variables|/Game/BluePrints/Main/Paddle/WB_DeathTimer.WB_DeathTimer_C|SetTime (Variables|Default|GetDeath%20Timer) _death))
          (:Finished
            (bind _outactors (Actor|GetAllActorsOfClass "/Game/BluePrints/Main/BP_BallSpawn.BP_BallSpawn_C"))
            (bind _asbp_ball_spawn (Utilities|Casting|CastToBP_BallSpawn (Utilities|Array|Get(acopy) _outactors)))
            (Default|SpawnBall _asbp_ball_spawn)
            (Widget|RemovefromParent (Variables|Default|GetDeath%20Timer))))))))

(event EventBeginPlay)

(event Collision|EventActorBeginOverlap
  (params (OtherActor :type Actor%20Object%20Reference)))

(event EventTick
  (params (DeltaSeconds :type Float%20%28single-precision%29)))

(fn ConstructionScript)