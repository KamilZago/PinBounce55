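; BP_Paddle is a Blueprint with left and right paddles that swing about the yaw of their own pivots, like flippers.
; LeftPaddle and RightPaddle play timelines from the start that drive yaw, while matching Reset events play separate timelines in reverse from the end.
; Both swing timelines share a PlaySound2D call for SC_Paddle on their Update pin, so it fires every update rather than once per swing.
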(event Custom|LeftPaddle
  (bind _pivotleft (Variables|Default|GetPivotLeft))
  (bind _relativerotation (Variables|/Script/Engine.SceneComponent|GetRelativeRotation _pivotleft))
  (bind (_roll _pitch) (Math|Rotator|BreakRotator _relativerotation))
  (bind _newtrack_0 (Timeline|LeftTime PlayFromStart)
    (:Update
      (Transformation|SetRelativeRotation _pivotleft (Math|Rotator|MakeRotator _roll _pitch _newtrack_0) false false)
      (Audio|PlaySound2D "/Game/BluePrints/Main/Sounds/SC_Paddle.SC_Paddle" 1.0 1.0 0.0 0 0))))

(event Custom|RightPaddle
  (bind _pivotright (Variables|Default|GetPivotRight))
  (bind _relativerotation (Variables|/Script/Engine.SceneComponent|GetRelativeRotation _pivotright))
  (bind (_roll _pitch) (Math|Rotator|BreakRotator _relativerotation))
  (bind _newtrack_0 (Timeline|RightTime PlayFromStart)
    (:Update
      (Transformation|SetRelativeRotation _pivotright (Math|Rotator|MakeRotator _roll _pitch _newtrack_0) false false)
      (Audio|PlaySound2D "/Game/BluePrints/Main/Sounds/SC_Paddle.SC_Paddle" 1.0 1.0 0.0 0 0))))

(event Custom|LeftPaddleReset
  (bind _pivotleft (Variables|Default|GetPivotLeft))
  (bind _relativerotation (Variables|/Script/Engine.SceneComponent|GetRelativeRotation _pivotleft))
  (bind (_roll _pitch) (Math|Rotator|BreakRotator _relativerotation))
  (bind _newtrack_0 (Timeline|Timeline ReverseFromEnd)
    (:Update
      (Transformation|SetRelativeRotation _pivotleft (Math|Rotator|MakeRotator _roll _pitch _newtrack_0) false false))))

(event Custom|RightPaddleReset
  (bind _pivotright (Variables|Default|GetPivotRight))
  (bind _relativerotation (Variables|/Script/Engine.SceneComponent|GetRelativeRotation _pivotright))
  (bind (_roll _pitch) (Math|Rotator|BreakRotator _relativerotation))
  (bind _newtrack_0 (Timeline|Timeline_0 ReverseFromEnd)
    (:Update
      (Transformation|SetRelativeRotation _pivotright (Math|Rotator|MakeRotator _roll _pitch _newtrack_0) false false))))

(fn ConstructionScript)