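; BP_Character is the character Blueprint that drives a scripted camera move and procedural camera shake.
; MoveCamera uses a timeline to move the actor to the first BP_CameraGoTo while widening the FOV and rotating the camera.
; A second timeline scales random unit vectors by strength to jitter the camera's relative location, once or looped for a given duration.
; BeginPlay and Tick are empty, and the in-graph calls to MoveCamera and CameraShake never run.
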(event Custom|CameraShakeStart
  (bind _shake1 (Timeline|Timeline PlayFromStart)
    (:Update
      (Transformation|SetRelativeLocation (Variables|Default|GetCamera) (* _shake1 (Math|Random|RandomUnitVector) (Variables|Default|GetStrengh)) false false))
    (:Finished
      (if (Variables|Default|Get?Loop)
        (Timeline|Timeline PlayFromStart)))))

(event Custom|CameraShakeStop
  (bind _shake1 (Timeline|Timeline Stop)
    (:Update
      (Transformation|SetRelativeLocation (Variables|Default|GetCamera) (* _shake1 (Math|Random|RandomUnitVector) (Variables|Default|GetStrengh)) false false))
    (:Finished
      (if (Variables|Default|Get?Loop)
        (Timeline|Timeline PlayFromStart)))))

(event Custom|CameraShake
  (params (Duration :type Float%20%28double-precision%29) (Strengh :type Integer))
  (CallFunction|CameraShakeStart)
  (Variables|Default|Set?Loop true)
  (Variables|Default|SetStrengh Strengh)
  (Utilities|FlowControl|Delay Duration)
  (CallFunction|CameraShakeStop)
  (Variables|Default|Set?Loop false))

(event Custom|SingleCameraShake
  (params (Strengh :type Integer))
  (Variables|Default|SetStrengh Strengh)
  (bind _shake1 (Timeline|Timeline PlayFromStart)
    (:Update
      (Transformation|SetRelativeLocation (Variables|Default|GetCamera) (* _shake1 (Math|Random|RandomUnitVector) (Variables|Default|GetStrengh)) false false))
    (:Finished
      (if (Variables|Default|Get?Loop)
        (Timeline|Timeline PlayFromStart)))))

(event Custom|MoveCamera
  (bind _self self)
  (bind _outactors (Actor|GetAllActorsOfClass "/Game/BluePrints/Main/BP_CameraGoTo.BP_CameraGoTo_C"))
  (Variables|Default|SetStart%20Location (Transformation|GetActorLocation _self))
  (bind _lerp (Timeline|CameraStart Play)
    (:Update
      (Transformation|SetActorLocation _self (Math|Vector|Lerp(Vector) (Variables|Default|GetStart%20Location) (Transformation|GetActorLocation (Utilities|Array|Get(acopy) _outactors)) _lerp) false false)
      (Camera|SetFieldOfView (Variables|Default|GetCamera) (Math|Float|Lerp 65.0 9e+01 _lerp))
      (Transformation|SetRelativeRotation (Variables|Default|GetCamera) (Math|Rotator|Lerp(Rotator) "-12.000000,0.000000,0.000000" "-70.000000,0.000000,0.000000" _lerp) false false))))

(event EventBeginPlay)

(event Collision|EventActorBeginOverlap
  (params (OtherActor :type Actor%20Object%20Reference)))

(event EventTick
  (params (DeltaSeconds :type Float%20%28single-precision%29)))

(fn ConstructionScript)