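; Enemy spawn point that spawns BP_Enemy of a random type at a random Y offset, keeping its own X, Z and rotation.
; StartGame enables Tick, which accumulates play time and derives a shrinking spawn interval from DefaultCzas and ZmianaCzasu, with a lower floor.
; Tick relies on Delay ignoring re-triggers while pending, so it acts as a repeating timer that calls Spawn.
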(event Custom|StartGame
  (Variables|Default|Set?Started true))

(event EventBeginPlay)

(event Collision|EventActorBeginOverlap
  (params (OtherActor :type Actor%20Object%20Reference)))

(event EventTick
  (params (DeltaSeconds :type Float%20%28single-precision%29))
  (if (Variables|Default|Get?Started)
    (bind _output_get (Variables|Default|Setczas%20gry (+ DeltaSeconds (Variables|Default|Getczas%20gry))))
    (if (< (- (Variables|Default|GetDefault%20czas) (* (Math|Float|Round _output_get) (Variables|Default|GetZmianaCzasu))) 0.1)
      (Utilities|FlowControl|Delay 0.1)
      (CallFunction|Spawn)
      (else
        (Utilities|FlowControl|Delay (- (Variables|Default|GetDefault%20czas) (* (Math|Float|Round _output_get) (Variables|Default|GetZmianaCzasu))))
        (CallFunction|Spawn)))))

(fn ConstructionScript)

(fn Spawn
  (bind _self self)
  (bind _returnvalue (Transformation|GetActorTransform _self))
  (bind (_location _rotation _scale) (Math|Transform|BreakTransform _returnvalue))
  (bind (_x _y _z) (Math|Vector|BreakVector _location))
  (Game|SpawnActorfromClass "/Game/BluePrints/Main/Enemy/BP_Enemy.BP_Enemy_C" (Math|Transform|MakeTransform (Math|Vector|MakeVector _x (Math|Random|RandomFloatinRange -1.7e+03 1.7e+03) _z) _rotation _scale) "Undefined" "MultiplyWithRoot" 0 (.OutItem (Utilities|Array|Random (Utilities|Array|MakeArray "NewEnumerator0" "NewEnumerator1" "NewEnumerator2"))) 0))