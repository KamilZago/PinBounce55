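; Enemy sphere that loses 1 HP per overlap with BP_MainBall and awards score when destroyed.
; On BeginPlay it looks up its Type in DT_Enemy to set size, damping, material, HP and score value; one Type also overlaps the Vehicle channel.
; Overlaps spawn a hit effect, while Tick polls for zero HP, then adds score through BP_Menager, spawns a death effect and destroys the actor.
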(event OnComponentBeginOverlap(Sphere)
  (params (OverlappedComponent :type Primitive%20Component%20Object%20Reference) (OtherActor :type Actor%20Object%20Reference) (OtherComp :type Primitive%20Component%20Object%20Reference) (OtherBodyIndex :type Integer) (bFromSweep :type Boolean) (SweepResult :type Hit%20Result%20Structure%20%28by%20ref%29))
  (bind _sphere (Variables|Default|GetSphere))
  (bind _returnvalue (Transformation|GetWorldTransform _sphere))
  (bind (_location _rotation) (Math|Transform|BreakTransform _returnvalue))
  ;[0.15 0 0 0.5] Smierc
  (Utilities|Casting|CastToBP_MainBall OtherActor)
  (Variables|Default|SetHP (- (Variables|Default|GetHP) 1))
  (Niagara|SpawnSystematLocation "/Game/BluePrints/Main/Particle/ES_EnemyHit.ES_EnemyHit" _location _rotation))

(event EventBeginPlay
  (bind _sphere (Variables|Default|GetSphere))
  (if (Utilities|Enum|Equal(Enum) (Variables|Default|GetType) "NewEnumerator1")
    (Collision|SetCollisionResponsetoChannel (Variables|Default|GetSphere) "ECC_Vehicle" "ECR_Overlap"))
  (bind _outrownames (DataTable|GetDataTableRowNames "/Game/BluePrints/Main/Enemy/DT_Enemy.DT_Enemy"))
  (for _array_element _outrownames
    (bind _returnvalue (Utilities|GetDataTableRow "/Game/BluePrints/Main/Enemy/DT_Enemy.DT_Enemy" _array_element)
      (:then
        (if (Utilities|Enum|Equal(Enum) (.Type (Utilities|Struct|BreakST_Enemy _returnvalue)) (Variables|Default|GetType))
          (Transformation|SetRelativeScale3D _sphere (Math|Vector|MakeVector (.Size (Utilities|Struct|BreakST_Enemy _returnvalue)) (.Size (Utilities|Struct|BreakST_Enemy _returnvalue)) (.Size (Utilities|Struct|BreakST_Enemy _returnvalue))))
          (Class|PrimitiveComponent|SetAngularDamping _sphere (.Damping (Utilities|Struct|BreakST_Enemy _returnvalue)))
          (Variables|Default|SetValue (.Value (Utilities|Struct|BreakST_Enemy _returnvalue)))
          (bind _returnvalue_2 (Rendering|Material|CreateDynamicMaterialInstance (.Material (Utilities|Struct|BreakST_Enemy _returnvalue)) "None" "None" :!class /Script/Engine.KismetMaterialLibrary))
          (Rendering|Material|SetMaterial _sphere 0 _returnvalue_2)
          (bind _output_get (Variables|Default|SetMaxHP (.HP (Utilities|Struct|BreakST_Enemy _returnvalue))))
          (Variables|Default|SetHP _output_get))))))

(event Collision|EventActorBeginOverlap
  (params (OtherActor :type Actor%20Object%20Reference)))

(event EventTick
  (params (DeltaSeconds :type Float%20%28single-precision%29))
  (bind _sphere (Variables|Default|GetSphere))
  (bind _returnvalue (Transformation|GetWorldTransform _sphere))
  (bind (_location _rotation) (Math|Transform|BreakTransform _returnvalue))
  ;[0.15 0 0 0.5] Smierc
  (if (<= (Variables|Default|GetHP) 0)
    (bind _outactors (Actor|GetAllActorsOfClass "/Game/Upgrades/BP_Menager.BP_Menager_C"))
    (Default|AddScore (Utilities|Array|Get(acopy) _outactors) (Variables|Default|GetValue))
    (Niagara|SpawnSystematLocation "/Game/BluePrints/Main/Particle/ES_EnemyDeath.ES_EnemyDeath" _location _rotation)
    (Actor|DestroyActor self)))

(fn ConstructionScript)